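; HUD Blueprint for an N-body octree scene that creates the on-screen UI and bootstraps the point simulation.
; The construction script calls Setup, which creates BP_ScreenUI and adds it to the viewport.
; BeginPlay spawns an OctreeSearch actor, generates its space points, enables its tick, and hands the actor to the widget.
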(event EventBeginPlay
  (bind _returnvalue (Game|SpawnActorfromClass "/Script/NBody.OctreeSearch" (Math|Transform|MakeTransform "0, 0, 0" "0, 0, 0" "1,1,1") "AlwaysSpawn" 0 0))
  (Class|OctreeSearch|CreateSpacePoints _returnvalue 2048 1e+04)
  (Actor|Tick|SetActorTickEnabled _returnvalue true)
  (Variables|/Game/HUD/BP_ScreenUI.BP_ScreenUI_C|SetOctree (Variables|Default|GetScreenWidget) _returnvalue))

(event EventBeginPlay)

(fn ConstructionScript
  (CallFunction|Setup))

(fn Setup
  (bind _returnvalue (UserInterface|CreateWidget "/Game/HUD/BP_ScreenUI.BP_ScreenUI_C"))
  (UserInterface|Viewport|AddtoViewport _returnvalue 0)
  (Variables|Default|SetScreenWidget _returnvalue))